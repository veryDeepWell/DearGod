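; BP_Home is a house actor that populates itself with BP_People and updates the game mode's score.
; After BeginPlay it uses timed up and down forces, stops simulating physics on hitting BP_Plane, then spawns people in a delayed loop, adding score until MaxPeople runs out.
; Trigger boxes teleport people to Box1 or destroy them with a score penalty.
; Cube overlaps toggle BP_Shadow's build state, switching it off while overlapping.
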(event `self.ReceiveBeginPlay`
  (bind _asbp_game_mode (cast `/Game/Blueprints/BP_GameMode` (`GameplayStatics.GetGameMode`)))
  (set `self.GameMode` _asbp_game_mode)
  (`PrimitiveComponent.AddForce` (`self.Cube`) (0.0 0.0 100000.0) "None" false)
  (`KismetSystemLibrary.Delay` 0.5)
  (`PrimitiveComponent.AddForce` (`self.Cube`) (0.0 0.0 -500000.0) "None" false))

(event `self.Cube.OnComponentHit`
  (params (HitComponent :type "PrimitiveComponent Object Reference") (OtherActor :type "Actor Object Reference") (OtherComp :type "PrimitiveComponent Object Reference") (NormalImpulse :type "Vector Structure") (Hit :type "HitResult Structure (by ref)"))
  (bind _returnvalue (`SceneComponent.K2_GetComponentToWorld` (`self.Cube`)))
  (cast `/Game/Blueprints/BP_Plane` OtherActor)
  (`PrimitiveComponent.SetSimulatePhysics` (`self.Cube`) false)
  (`KismetSystemLibrary.Delay` 2.0 :!label _label)
  (`/Game/Blueprints/BP_GameMode.AddScore` (`self.GameMode`) 1)
  (`/Engine/EditorBlueprintResources/StandardMacros.DecrementFloat` (`self.MaxPeople`)
    (:`  `
      (`|SpawnActorFromClass` "/Game/Blueprints/BP_People.BP_People_C" (`KismetMathLibrary.MakeTransform` (`KismetMathLibrary.MakeVector` (.x (.location _returnvalue)) (+ (.y (.location _returnvalue)) 200.0) (+ (.z (.location _returnvalue)) 100.0))) "Undefined" "MultiplyWithRoot" null null)
      (if (not (<= (`self.MaxPeople`) 0.0))
        (goto _label)))))

(event `self.Box2.OnComponentBeginOverlap`
  (params (OverlappedComponent :type "PrimitiveComponent Object Reference") (OtherActor :type "Actor Object Reference") (OtherComp :type "PrimitiveComponent Object Reference") (OtherBodyIndex :type Integer) (bFromSweep :type Boolean) (SweepResult :type "HitResult Structure (by ref)"))
  (bind _asbp_people (cast `/Game/Blueprints/BP_People` OtherActor))
  (`/Game/Blueprints/BP_GameMode.AddScore` (`self.GameMode`) -1)
  (`self.K2_DestroyActor` _asbp_people))

(event `self.Box.OnComponentBeginOverlap`
  (params (OverlappedComponent :type "PrimitiveComponent Object Reference") (OtherActor :type "Actor Object Reference") (OtherComp :type "PrimitiveComponent Object Reference") (OtherBodyIndex :type Integer) (bFromSweep :type Boolean) (SweepResult :type "HitResult Structure (by ref)"))
  (bind _asbp_people (cast `/Game/Blueprints/BP_People` OtherActor))
  (`SceneComponent.K2_SetWorldLocation` (`/Game/Blueprints/BP_People.Cube` _asbp_people) (`SceneComponent.K2_GetComponentLocation` (`self.Box1`)) false true))

(event `self.Cube.OnComponentBeginOverlap`
  (params (OverlappedComponent :type "PrimitiveComponent Object Reference") (OtherActor :type "Actor Object Reference") (OtherComp :type "PrimitiveComponent Object Reference") (OtherBodyIndex :type Integer) (bFromSweep :type Boolean) (SweepResult :type "HitResult Structure (by ref)"))
  (bind _asbp_shadow (cast `/Game/Blueprints/BP_Shadow` OtherActor))
  (`/Game/Blueprints/BP_Shadow.OffBuild` _asbp_shadow))

(event `self.Cube.OnComponentEndOverlap`
  (params (OverlappedComponent :type "PrimitiveComponent Object Reference") (OtherActor :type "Actor Object Reference") (OtherComp :type "PrimitiveComponent Object Reference") (OtherBodyIndex :type Integer))
  (bind _asbp_shadow (cast `/Game/Blueprints/BP_Shadow` OtherActor))
  (`/Game/Blueprints/BP_Shadow.OnBuild` _asbp_shadow))

(fn `UserConstructionScript`)