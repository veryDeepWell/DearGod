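; Game mode that tracks the score and shows it through a BP_Score HUD widget.
; On BeginPlay it sets game-only input, creates the widget and resets the displayed score to zero.
; AddScore accumulates points and updates the score text via SetScore.
; On reaching MaxScore it switches to UI-only input, shows the mouse cursor and reveals the widget's God element as an end state.
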(event `self.ReceiveBeginPlay`
  (`WidgetBlueprintLibrary.SetInputMode_GameOnly` (`GameplayStatics.GetPlayerController` 0))
  (bind _returnvalue (`|CreateWidget` "/Game/Blueprints/BP_Score.BP_Score_C"))
  (`UserWidget.AddToViewport` _returnvalue 0)
  (set `self.Widget` _returnvalue)
  (`self.SetScore` 0))

(fn `AddScore`
  (params (Ante :type Integer))
  (bind _returnvalue (`GameplayStatics.GetPlayerController` 0))
  (bind _output_get (set `self.Score` (+ (`self.Score`) Ante)))
  (if (>= _output_get (`self.MaxScore`))
    (`self.SetScore` _output_get)
    (bind _asbp_score (cast `/Game/Blueprints/BP_Score` (`self.Widget`)))
    (`WidgetBlueprintLibrary.SetInputMode_UIOnlyEx` _returnvalue null "DoNotLock" true)
    (set `PlayerController.bShowMouseCursor` true _returnvalue)
    (set `Widget.Visibility` "Visible" (`/Game/Blueprints/BP_Score.God` _asbp_score))
    (else
      (`self.SetScore` _output_get))))

(fn `SetScore`
  (params (Peoples :type Integer))
  (bind _asbp_score (cast `/Game/Blueprints/BP_Score` (`self.Widget`)))
  (set `TextBlock.Text` (`|GenericToText` Peoples) (`/Game/Blueprints/BP_Score.Score_Text` _asbp_score)))

(fn `UserConstructionScript`)