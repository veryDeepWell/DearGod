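; BP_People is an actor whose Cube component hops around repeatedly, apparently standing in for a person.
; On BeginPlay it waits for JumpDelay, then gives the cube a starting upward impulse with a random positive sideways offset.
; Each component hit on the cube adds another impulse of JumpHeight upward and a random offset in either horizontal direction, so physics collisions keep the hopping going.
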(event `self.ReceiveBeginPlay`
  (`KismetSystemLibrary.Delay` (`self.JumpDelay`))
  (`PrimitiveComponent.AddImpulse` (`self.Cube`) (`KismetMathLibrary.MakeVector` (`KismetMathLibrary.RandomFloatInRange` 0.0 (`self.Offset`)) (`KismetMathLibrary.RandomFloatInRange` 0.0 (`self.Offset`)) 100.0) "None" false))

(event `self.Cube.OnComponentHit`
  (params (HitComponent :type "PrimitiveComponent Object Reference") (OtherActor :type "Actor Object Reference") (OtherComp :type "PrimitiveComponent Object Reference") (NormalImpulse :type "Vector Structure") (Hit :type "HitResult Structure (by ref)"))
  (`PrimitiveComponent.AddImpulse` (`self.Cube`) (`KismetMathLibrary.MakeVector` (`KismetMathLibrary.RandomFloatInRange` (* (`self.Offset`) -1.0) (`self.Offset`)) (`KismetMathLibrary.RandomFloatInRange` (* (`self.Offset`) -1.0) (`self.Offset`)) (`self.Jump Height`)) "None" false))

(fn `UserConstructionScript`)