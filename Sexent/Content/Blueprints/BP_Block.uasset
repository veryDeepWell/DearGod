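; BP_Block is a block actor that blocks building wherever a BP_Shadow actor overlaps it.
; On BeginPlay it applies its Mesh and Material variables to the Cube component.
; The Cube's overlap events call OffBuild on a BP_Shadow when it enters and OnBuild when it leaves, with no count of other blocks still overlapping.
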(event `self.ReceiveBeginPlay`
  (`StaticMeshComponent.SetStaticMesh` (`self.Cube`) (`self.Mesh`))
  (`PrimitiveComponent.SetMaterial` (`self.Cube`) 0 (`self.Material`)))

(event `self.Cube.OnComponentBeginOverlap`
  (params (OverlappedComponent :type "PrimitiveComponent Object Reference") (OtherActor :type "Actor Object Reference") (OtherComp :type "PrimitiveComponent Object Reference") (OtherBodyIndex :type Integer) (bFromSweep :type Boolean) (SweepResult :type "HitResult Structure (by ref)"))
  (bind _asbp_shadow (cast `/Game/Blueprints/BP_Shadow` OtherActor))
  (`/Game/Blueprints/BP_Shadow.OffBuild` _asbp_shadow))

(event `self.Cube.OnComponentEndOverlap`
  (params (OverlappedComponent :type "PrimitiveComponent Object Reference") (OtherActor :type "Actor Object Reference") (OtherComp :type "PrimitiveComponent Object Reference") (OtherBodyIndex :type Integer))
  (bind _asbp_shadow (cast `/Game/Blueprints/BP_Shadow` OtherActor))
  (`/Game/Blueprints/BP_Shadow.OnBuild` _asbp_shadow))

(fn `UserConstructionScript`)