(event `self.ReceiveBeginPlay`
  (`PrimitiveComponent.SetMaterial` (`self.Cube`) 0 "/Game/Materials/M_GreenShadow.M_GreenShadow"))

(event `InputAxis|Daun`
  (params (AxisValue :type "Float (single-precision)"))
  (`SceneComponent.K2_AddLocalOffset` (`self.Cube`) (`KismetMathLibrary.MakeVector` (* AxisValue (`self.Speed`))) true false))

(event `InputAction|SetShadow`
  (params (Key :type "Key Structure"))
  (:`Pressed`
    (for _array_element (`PrimitiveComponent.GetOverlappingActors` (`self.Cube4`) "/Game/Blueprints/BP_Home.BP_Home_C")
      (bind _asbp_home (cast `/Game/Blueprints/BP_Home` _array_element)))))

(event `InputAxis|Autism`
  (params (AxisValue :type "Float (single-precision)"))
  (`SceneComponent.K2_AddLocalOffset` (`self.Cube`) (`KismetMathLibrary.MakeVector` 0.0 (* AxisValue (`self.Speed`))) true false))

(event `InputAxis|Zoom`
  (params (AxisValue :type "Float (single-precision)"))
  (bind _camera (`self.Camera`))
  (bind _speedzoom (`self.SpeedZoom`))
  (`SceneComponent.K2_AddLocalOffset` _camera (`KismetMathLibrary.MakeVector` (* AxisValue 8.0 _speedzoom) 0.0 (* AxisValue -16.0 _speedzoom)) false false)
  (`SceneComponent.K2_AddLocalRotation` _camera (`KismetMathLibrary.MakeRotator` 0.0 (* AxisValue 0.2 (`self.SpeedZoom`))) false false))

(event `InputAction|Build`
  (params (Key :type "Key Structure"))
  (bind _cube (`self.Cube`))
  (bind (_returnvalue_x _returnvalue_y _returnvalue_z) (`KismetMathLibrary.BreakVector` (`SceneComponent.K2_GetComponentLocation` _cube)))
  (:`Pressed`
    (if (`self.CanSpawn`)
      (`self.OffBuild`)
      (`|SpawnActorFromClass` "/Game/Blueprints/BP_Home.BP_Home_C" (`KismetMathLibrary.MakeTransform` (`KismetMathLibrary.MakeVector` _returnvalue_x _returnvalue_y (+ _returnvalue_z 1000.0)) (`SceneComponent.K2_GetComponentRotation` _cube)) "Undefined" "MultiplyWithRoot" null null)
      (`KismetSystemLibrary.Delay` 2.0)
      (if (`KismetArrayLibrary.Array_IsEmpty` (`PrimitiveComponent.GetOverlappingActors` (`self.Cube`) "/Game/Blueprints/BP_Home.BP_Home_C"))
        (`self.OnBuild` :!label _label)
        (elif (`KismetArrayLibrary.Array_IsEmpty` (`PrimitiveComponent.GetOverlappingActors` (`self.Cube`) "/Game/Blueprints/BP_Block.BP_Block_C"))
          (goto _label))))))

(event `InputAxis|Rotate`
  (params (AxisValue :type "Float (single-precision)"))
  (bind _returnvalue (* AxisValue (`self.SpeedRotate`)))
  (`SceneComponent.K2_AddWorldRotation` (`self.Cube`) (`KismetMathLibrary.MakeRotator` 0.0 0.0 _returnvalue) false false)
  (`SceneComponent.K2_AddLocalRotation` (`self.wa`) (`KismetMathLibrary.MakeRotator` 0.0 0.0 (* _returnvalue -1.0)) false false))

(event `Key|Up`
  (params (Key :type "Key Structure"))
  (:`Pressed`
    (`SceneComponent.K2_SetWorldRotation` :`self` (`self.Cube`))
    (`SceneComponent.K2_SetRelativeRotation` (`self.wa`) (`KismetMathLibrary.MakeRotator` 74.0 0.0 120.0) false false)))

(event `Key|Down`
  (params (Key :type "Key Structure"))
  (:`Pressed`
    (`SceneComponent.K2_SetWorldRotation` (`self.Cube`) (struct :`Yaw` 180.0) false false)
    (`SceneComponent.K2_SetRelativeRotation` (`self.wa`) (`KismetMathLibrary.MakeRotator` 74.0 180.0 120.0) false false)))

(event `Key|Left`
  (params (Key :type "Key Structure"))
  (:`Pressed`
    (`SceneComponent.K2_SetWorldRotation` (`self.Cube`) (`KismetMathLibrary.MakeRotator` 0.0 0.0 -90.0) false false)
    (`SceneComponent.K2_SetRelativeRotation` (`self.wa`) (`KismetMathLibrary.MakeRotator` 74.0 -90.0 120.0) false false)))

(event `Key|Right`
  (params (Key :type "Key Structure"))
  (:`Pressed`
    (`SceneComponent.K2_SetWorldRotation` (`self.Cube`) (struct :`Yaw` 90.0) false false)
    (`SceneComponent.K2_SetRelativeRotation` (`self.wa`) (`KismetMathLibrary.MakeRotator` 74.0 90.0 120.0) false false)))

(fn `OffBuild`
  (set `self.CanSpawn` false)
  (`PrimitiveComponent.SetMaterial` (`self.Cube`) 0 "/Game/Materials/M_RedShadow.M_RedShadow"))

(fn `OnBuild`
  (set `self.CanSpawn` true)
  (`PrimitiveComponent.SetMaterial` (`self.Cube`) 0 "/Game/Materials/M_GreenShadow.M_GreenShadow"))

(fn `UserConstructionScript`)