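; Player-controlled building placement ghost that moves, rotates and zooms its camera, and spawns BP_House on the Build input.
; Axis inputs sweep and turn the Cube while counter-rotating Wa; arrow keys snap both to fixed orientations.
; Houses spawn above the Scene component when CanSpawn is set, followed by a red-shadow cooldown that ends only if no BP_BlockObject overlaps.
; Tab freezes time and shows the game mode widget's STOP element with UI-only input.
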(event `InputAxis|Daun`
  (params (AxisValue :type "Float (single-precision)"))
  ; Передвижение
  (`SceneComponent.K2_AddLocalOffset` (`self.Cube`) (`KismetMathLibrary.MakeVector` (* AxisValue (`self.Speed`))) true false))

(event `self.ReceiveBeginPlay`
  ; Comment
  (`PrimitiveComponent.SetMaterial` (`self.Cube`) 0 "/Game/Materials/M_GreenShadow.M_GreenShadow"))

(event `InputAction|Build`
  (params (Key :type "Key Structure"))
  (bind _scene (`self.Scene`))
  (bind (_returnvalue_roll _returnvalue_pitch _returnvalue_yaw) (`KismetMathLibrary.BreakRotator` (`SceneComponent.K2_GetComponentRotation` _scene)))
  (bind (_returnvalue_x _returnvalue_y _returnvalue_z) (`KismetMathLibrary.BreakVector` (`SceneComponent.K2_GetComponentLocation` _scene)))
  ; Строительство
  (:`Pressed`
    (if (`self.CanSpawn`)
      (`self.OffBuild`)
      (`|SpawnActorFromClass` "/Game/Blueprints/BlockObject/BP_House.BP_House_C" (`KismetMathLibrary.MakeTransform` (`KismetMathLibrary.MakeVector` _returnvalue_x _returnvalue_y (+ _returnvalue_z 1000.0)) (`KismetMathLibrary.MakeRotator` _returnvalue_roll _returnvalue_pitch (+ _returnvalue_yaw 180.0))) "Undefined" "MultiplyWithRoot" null null)
      (`KismetSystemLibrary.Delay` 2.0)
      (`self.OnBuild`))))

(event `InputAxis|Autism`
  (params (AxisValue :type "Float (single-precision)"))
  ; Передвижение
  (`SceneComponent.K2_AddLocalOffset` (`self.Cube`) (`KismetMathLibrary.MakeVector` 0.0 (* AxisValue (`self.Speed`))) true false))

(event `Key|Tab`
  (params (Key :type "Key Structure"))
  (bind _returnvalue (`GameplayStatics.GetPlayerController` 0))
  (:`Pressed`
    (`GameplayStatics.SetGlobalTimeDilation` 0.0)
    (`WidgetBlueprintLibrary.SetInputMode_UIOnlyEx` _returnvalue null)
    (set `PlayerController.bShowMouseCursor` true _returnvalue)
    (bind _asbp_game_mode (cast `/Game/Blueprints/GameModes/BP_GameMode` (`GameplayStatics.GetGameMode`)))
    (set `Widget.Visibility` "Visible" (`/Game/Blueprints/Widgets/BP_Score.STOP` (`/Game/Blueprints/GameModes/BP_GameMode.Widget` _asbp_game_mode)))))

(event `InputAxis|Zoom`
  (params (AxisValue :type "Float (single-precision)"))
  (bind _camera (`self.Camera`))
  (bind _speedzoom (`self.SpeedZoom`))
  ; Камера
  (`SceneComponent.K2_AddLocalOffset` _camera (`KismetMathLibrary.MakeVector` (* AxisValue 8.0 _speedzoom) 0.0 (* AxisValue -16.0 _speedzoom)) false false)
  (`SceneComponent.K2_AddLocalRotation` _camera (`KismetMathLibrary.MakeRotator` 0.0 (* AxisValue 0.2 (`self.SpeedZoom`))) false false))

(event `InputAxis|Rotate`
  (params (AxisValue :type "Float (single-precision)"))
  (bind _returnvalue (* AxisValue (`self.SpeedRotate`)))
  ; Поворот
  (`SceneComponent.K2_AddWorldRotation` (`self.Cube`) (`KismetMathLibrary.MakeRotator` 0.0 0.0 _returnvalue) false false)
  (`SceneComponent.K2_AddLocalRotation` (`self.wa`) (`KismetMathLibrary.MakeRotator` 0.0 0.0 (* _returnvalue -1.0)) false false))

(event `Key|Up`
  (params (Key :type "Key Structure"))
  ; Поворот
  (:`Pressed`
    (`SceneComponent.K2_SetWorldRotation` :`self` (`self.Cube`))
    (`SceneComponent.K2_SetRelativeRotation` (`self.wa`) (`KismetMathLibrary.MakeRotator` 74.0 0.0 120.0) false false)))

(event `Key|Down`
  (params (Key :type "Key Structure"))
  ; Поворот
  (:`Pressed`
    (`SceneComponent.K2_SetWorldRotation` (`self.Cube`) (struct :`Yaw` 180.0) false false)
    (`SceneComponent.K2_SetRelativeRotation` (`self.wa`) (`KismetMathLibrary.MakeRotator` 74.0 180.0 120.0) false false)))

(event `Key|Left`
  (params (Key :type "Key Structure"))
  ; Поворот
  (:`Pressed`
    (`SceneComponent.K2_SetWorldRotation` (`self.Cube`) (`KismetMathLibrary.MakeRotator` 0.0 0.0 -90.0) false false)
    (`SceneComponent.K2_SetRelativeRotation` (`self.wa`) (`KismetMathLibrary.MakeRotator` 74.0 -90.0 120.0) false false)))

(event `Key|Right`
  (params (Key :type "Key Structure"))
  ; Поворот
  (:`Pressed`
    (`SceneComponent.K2_SetWorldRotation` (`self.Cube`) (struct :`Yaw` 90.0) false false)
    (`SceneComponent.K2_SetRelativeRotation` (`self.wa`) (`KismetMathLibrary.MakeRotator` 74.0 90.0 120.0) false false)))

(fn `OffBuild`
  (set `self.CanSpawn` false)
  (`PrimitiveComponent.SetMaterial` (`self.Cube`) 0 "/Game/Materials/M_RedShadow.M_RedShadow"))

(fn `OnBuild`
  (if (`KismetArrayLibrary.Array_IsEmpty` (`PrimitiveComponent.GetOverlappingActors` (`self.Cube`) "/Game/Blueprints/BlockObject/BP_BlockObject.BP_BlockObject_C"))
    (set `self.CanSpawn` true)
    (`PrimitiveComponent.SetMaterial` (`self.Cube`) 0 "/Game/Materials/M_GreenShadow.M_GreenShadow")))

(fn `UserConstructionScript`)